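; Game mode that manages dedicated server session lifecycle and player tracking through GI_Vivox.
; On BeginPlay it enables seamless travel and, on dedicated servers, registers, logs in and binds session-removal results.
; Logins and logouts update a controller list and notify BP_GameState.
; When the last player leaves, room servers remove their session, retrying on failure before shutdown, while other servers shut down directly.
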(event `ShutdownServer`
  (bind _asgi_vivox (cast `GI_Vivox` (`GameplayStatics.GetGameInstance`) :!pure true))
  (bind _returnvalue (`GI_Vivox.IsRoomServer` _asgi_vivox))
  (if _returnvalue
    (`GI_Vivox.ServerRemoveGameSession` _asgi_vivox)
    (else
      (`GI_Vivox.Shutdown` (cast `GI_Vivox` (`GameplayStatics.GetGameInstance`) :!pure true) :!label _label))))

(event `HandleShutdownServer`
  (params (isSessionRemoved :type Boolean))
  (if isSessionRemoved
    (goto _label)
    (else
      (`GI_Vivox.ServerRemoveGameSession` (cast `GI_Vivox` (`GameplayStatics.GetGameInstance`) :!pure true)))))

(event `self.ReceiveBeginPlay`
  (set `self.bUseSeamlessTravel` true)
  (if (`KismetSystemLibrary.IsDedicatedServer`)
    (`GI_Vivox.ServerRegistrationAndLogin` (cast `GI_Vivox` (`GameplayStatics.GetGameInstance`) :!pure true))
    (set `self.GameInstanceRef` (cast `GI_Vivox` (`GameplayStatics.GetGameInstance`) :!pure true))
    (add `GI_Vivox.SessionRemoved` (cast `GI_Vivox` (`GameplayStatics.GetGameInstance`) :!pure true) (delegate `HandleShutdownServer`))))

(event `RemoveIfEmptySession`
  (`GI_Vivox.ServerRemoveGameSession` (cast `GI_Vivox` (`GameplayStatics.GetGameInstance`) :!pure true)))

(event `self.K2_PostLogin`
  (params (NewPlayer :type "PlayerController Object Reference"))
  (`KismetArrayLibrary.Array_Add` (`self.ActivePlayerControllers`) NewPlayer)
  (`/Game/BP_GameState.VerifyPlayerInitialisation` (cast `/Game/BP_GameState` (`GameplayStatics.GetGameState`) :!pure true) NewPlayer))

(event `self.K2_OnLogout`
  (params (ExitingController :type "Controller Object Reference"))
  (bind _activeplayercontrollers (`self.ActivePlayerControllers`))
  (`KismetSystemLibrary.PrintString` "OnLogout function fired." true true (struct :`G` 0.66 :`B` 1.0 :`A` 1.0) 20.0)
  (`KismetArrayLibrary.Array_RemoveItem` _activeplayercontrollers (cast `PlayerController` ExitingController :!pure true))
  (`/Engine/EditorBlueprintResources/StandardMacros.CompareInt` (`KismetArrayLibrary.Array_Length` _activeplayercontrollers)
    (:`>`
      (`KismetSystemLibrary.PrintString` "OnLogout: PlayerControllers > 0" true true (struct :`G` 0.66 :`B` 1.0 :`A` 1.0) 20.0)
      (`/Game/BP_GameState.RemovePlayer` (cast `/Game/BP_GameState` (`GameplayStatics.GetGameState`) :!pure true)))
    (:`==`
      (`self.ShutdownServer`))))

(event `/Game/BP_Registration.RegisterIncomingPlayer`
  (params (Username :type String))
  (`self.RegisterNewPlayer` Username))

(event `/Game/BP_Registration.DeregisterLeavingPlayer`
  (params (Username :type String))
  (`self.DeregisterPlayer` Username))

(fn `UserConstructionScript`)