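; Player state Blueprint that stores a player's IP details and an IsOwner flag, intended to carry them across level changes.
; CopyProperties and OverrideWith copy both values between old and new player states, with CopyProperties also calling a SetValues event, and print debug logs.
; The graph marks this copying as deprecated and non-functional, noting that the Game Instance is used instead.
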(event `SetValues`
  (params (IpDetails :type String) (isOwner :type Boolean))
  ;[1 0.9408 0] [DEPRECATED] Copying properties between levels (not functional: using Game Instance instead)
  (set `self.IpDetails` IpDetails)
  (bind _output_get (set `self.isOwner` isOwner))
  (`KismetSystemLibrary.PrintString` (`KismetStringLibrary.Concat_StrStr` "[PlayerState: CopyProperties] Server isOwner = " (`KismetStringLibrary.Conv_BoolToString` _output_get))))

(event `self.ReceiveCopyProperties`
  (params (NewPlayerState :type "PlayerState Object Reference"))
  (bind _isowner (`self.isOwner`))
  (bind _ipdetails (`self.IpDetails`))
  ;[1 0.9408 0] [DEPRECATED] Copying properties between levels (not functional: using Game Instance instead)
  (bind _asbp_player_state (cast `/Game/BP_PlayerState` NewPlayerState))
  (set `/Game/BP_PlayerState.IpDetails` _ipdetails _asbp_player_state)
  (set `/Game/BP_PlayerState.isOwner` _isowner _asbp_player_state)
  (`KismetSystemLibrary.PrintString` (`KismetStringLibrary.Concat_StrStr` "[PlayerState: CopyProperties] Client isOwner = " (`KismetStringLibrary.Conv_BoolToString` _isowner)))
  (`self.SetValues` _asbp_player_state _ipdetails _isowner))

(event `self.ReceiveOverrideWith`
  (params (OldPlayerState :type "PlayerState Object Reference"))
  ;[1 0.9408 0] [DEPRECATED] Copying properties between levels (not functional: using Game Instance instead)
  (bind _asbp_player_state (cast `/Game/BP_PlayerState` OldPlayerState))
  (set `self.IpDetails` (`/Game/BP_PlayerState.IpDetails` _asbp_player_state))
  (bind _isowner (`/Game/BP_PlayerState.isOwner` _asbp_player_state))
  (set `self.isOwner` _isowner)
  (`KismetSystemLibrary.PrintString` (`KismetStringLibrary.Concat_StrStr` "[PlayerState: OverrideWith] Client isOwner = " (`KismetStringLibrary.Conv_BoolToString` _isowner))))

(fn `SetIpDetails`
  (params (IpDetails :type String))
  (set `self.IpDetails` IpDetails))

(fn `UserConstructionScript`)