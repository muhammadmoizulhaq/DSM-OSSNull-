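; Game State that tracks players joining and leaving the server and updates client player lists.
; Waits for a new player's ThirdPersonCharacter and name, then registers it and multicasts it to each client's chat widget, also via NewPlayer's OnRep.
; GetPlayerNames gathers names from PlayerArray on clients, restarting when one is blank.
; Separate events handle deregistration, list removal and session list refresh through a GameInstance subsystem.
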(event `Server_DeregisterPlayer`
  (params (Username :type String))
  ;[1 1 1] Deregistering players leaving the server
  (`/Game/BP_Registration.DeregisterLeavingPlayer` Username))

(event `DelayList`
  ;[1 1 1] Misc
  (`KismetSystemLibrary.Delay` 0.5)
  (`KismetSystemLibrary.PrintString` "New player name still unassigned."))

(event `VerifyPlayerInitialisation`
  (params (NewPlayer :type "PlayerController Object Reference"))
  (bind _playerarray (`self.PlayerArray`))
  (bind (_asthird_person_character _bsuccess) (cast `/Game/ThirdPersonCPP/Blueprints/ThirdPersonCharacter` (`Controller.K2_GetPawn` (`self.NewPlayerControllerRef`)) :!pure true))
  (bind _playername (`/Game/ThirdPersonCPP/Blueprints/ThirdPersonCharacter.PlayerName` _asthird_person_character))
  (bind _playername_2 (`/Game/ThirdPersonCPP/Blueprints/ThirdPersonCharacter.PlayerName` (cast `/Game/ThirdPersonCPP/Blueprints/ThirdPersonCharacter` (`PlayerState.PawnPrivate` (`|GetArrayItem` _playerarray (`KismetArrayLibrary.Array_Find` _playerarray (`Controller.PlayerState` NewPlayer)))) :!pure true)))
  (bind _returnvalue (select `bool` (`KismetStringLibrary.EqualEqual_StrStr` _playername) :`false` _playername :`true` _playername_2))
  ;[1 1 1] Incoming player: Waiting for intialisation & multicasting new player's name
  ;;[1 1 1] Handling & waiting for player intialisation
  (set `self.NewPlayerControllerRef` NewPlayer)
  (if _bsuccess :!label _label
    (`KismetSystemLibrary.PrintString` (`KismetStringLibrary.Concat_StrStr` "GAME STATE NAME: " _playername_2 "    DIRECT PC NAME: " _playername))
    (if (`KismetStringLibrary.EqualEqual_StrStr` _returnvalue) :!label _label_2
      (if (> (`KismetArrayLibrary.Array_Length` (`self.PlayerArray`)) 0)
        (goto _label_2))
      (else
        (bind _output_get (set `self.NewPlayer` _returnvalue))
        (`self.Multicast_AddPlayerToClients` _output_get)
        (`/Game/BP_Registration.RegisterIncomingPlayer` _output_get)))
    (else
      (`KismetSystemLibrary.Delay` 0.01)
      (goto _label))))

(event `DeregisterPlayer`
  (params (Username :type String))
  ;[1 1 1] Deregistering players leaving the server
  (bind _output_get (set `self.LeavingPlayer` Username))
  (`self.Server_DeregisterPlayer` _output_get))

(event `RefreshServersList`
  ;[1 1 1] Misc
  (`GameInstanceSubsystemSessions.RefreshSessionsList` (subsystem `GameInstanceSubsystemSessions`)))

(event `Multicast_AddPlayerToClients`
  (params (Name :type String))
  (bind _wbp_chat_ref (`/Game/ThirdPersonCPP/Blueprints/ThirdPersonCharacter.WBP_Chat_Ref` (cast `/Game/ThirdPersonCPP/Blueprints/ThirdPersonCharacter` (`GameplayStatics.GetPlayerCharacter` 0) :!pure true)))
  ;[1 1 1] Incoming player: Waiting for intialisation & multicasting new player's name
  ;;[1 1 1] Multicasting player name to clients
  (`KismetSystemLibrary.PrintString` "Multicast GameState: AddPlayer function fired." true true (struct :`G` 0.66 :`B` 1.0 :`A` 1.0) 20.0)
  (`/Engine/EditorBlueprintResources/ActorMacros.Switch Has Authority`
    (:`Authority`
      (`KismetSystemLibrary.PrintString` "[SERVER] GameState: Adding player to widget." true true (struct :`G` 0.66 :`B` 1.0 :`A` 1.0) 20.0))
    (:`Remote`
      (`/Engine/EditorBlueprintResources/StandardMacros.IsValid` _wbp_chat_ref :!label _label_3
        (:`Is Valid`
          (`/Game/UI/WBP_GlobalChat.AddPlayerNameToList` _wbp_chat_ref Name))
        (:`Is Not Valid`
          (`KismetSystemLibrary.Delay` 0.5)
          (goto _label_3))))))

(event `RemovePlayer`
  ;[1 1 1] Remove Player from players list
  (`KismetSystemLibrary.PrintString` "Multicast GameState: RemovePlayer function fired." true true (struct :`G` 0.66 :`B` 1.0 :`A` 1.0) 20.0)
  (`/Engine/EditorBlueprintResources/ActorMacros.Switch Has Authority`
    (:`Authority`
      (`KismetSystemLibrary.PrintString` "GameState: Switch HAS AUTHORITY." true true (struct :`G` 0.66 :`B` 1.0 :`A` 1.0) 20.0))
    (:`Remote`
      (`KismetSystemLibrary.PrintString` "GameState: Switch has NO AUTHORITY." true true (struct :`G` 0.66 :`B` 1.0 :`A` 1.0) 20.0)
      (`/Game/ThirdPersonCPP/Blueprints/ThirdPersonCharacter.RemovePlayerNameFromList` (cast `/Game/ThirdPersonCPP/Blueprints/ThirdPersonCharacter` (`GameplayStatics.GetPlayerCharacter` 0) :!pure true)))))

(fn `GetPlayerNames`
  (returns (AllPlayerNames :type "Array of String"))
  (locals (PlayerNames :type "Array of String"))
  (for _array_element (`GameStateBase.PlayerArray` (`GameplayStatics.GetGameState`))
    (`/Engine/EditorBlueprintResources/ActorMacros.Switch Has Authority`
      (:`Remote`
        (bind _playername (`/Game/ThirdPersonCPP/Blueprints/ThirdPersonCharacter.PlayerName` (cast `/Game/ThirdPersonCPP/Blueprints/ThirdPersonCharacter` (`PlayerState.PawnPrivate` _array_element) :!pure true)))
        (if (`KismetStringLibrary.EqualEqual_StrStr` _playername)
          (`self.DelayList`)
          (`KismetArrayLibrary.Array_Clear` (`local.PlayerNames`))
          (bind _allplayernames (`self.GetPlayerNames`))
          (return _allplayernames)
          (else
            (`KismetSystemLibrary.PrintString` (`KismetStringLibrary.Concat_StrStr` "Adding player: " _playername) true true (struct :`R` 0.559079 :`G` 1.0 :`A` 1.0) 20.0)
            (`KismetArrayLibrary.Array_Add` (`local.PlayerNames`) _playername))))))
  (return (`local.PlayerNames`)))

(fn `OnRep_NewPlayer`
  (`self.Multicast_AddPlayerToClients` (`self.NewPlayer`)))

(fn `UserConstructionScript`)